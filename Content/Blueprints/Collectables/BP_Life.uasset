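; BP_Life is an extra-life collectable that spins in place until the player picks it up.
; A Rotation timeline drives the yaw of the Centre component and restarts itself whenever it finishes, giving a continuous spin.
; On overlap with BP_Player, it checks the life count in BP_GameInstance and, if below the maximum, calls ViePlus and destroys itself; otherwise it stays in the level.
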(event EventBeginPlay
  (bind _centre (Variables|Default|GetCentre))
  (bind _returnvalue (Transformation|GetWorldRotation _centre))
  ;[1 1 1] Animation
  (bind _rotation (Timeline|Rotation Play)
    (:Update
      (Transformation|SetWorldLocationAndRotation _centre (Transformation|GetWorldLocation _centre) (Math|Rotator|MakeRotator (.roll _returnvalue) (.pitch _returnvalue) _rotation) false false))
    (:Finished
      (Utilities|FlowControl|Delay 0.0)
      (Timeline|Rotation PlayFromStart))))

(event EventTick
  (params (DeltaSeconds :type Float%20%28single-precision%29)))

(event Collision|EventActorBeginOverlap
  (params (OtherActor :type Actor%20Object%20Reference))
  ;[1 1 1] Collection
  (Utilities|Casting|CastToBP_Player OtherActor)
  (bind _asbp_game_instance (Utilities|Casting|CastToBP_GameInstance (Game|GetGameInstance)))
  (if (< (Variables|/Script/Platformer_3D_Action.Platformer_GameInstance|Getm_Life _asbp_game_instance) (Variables|/Script/Platformer_3D_Action.Platformer_GameInstance|Getm_Max_Life _asbp_game_instance))
    (Class|PlatformerGameInstance|ViePlus _asbp_game_instance)
    (Actor|DestroyActor)))

(fn ConstructionScript)