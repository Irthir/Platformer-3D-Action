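; Projectile actor that damages whatever it hits and removes itself afterwards or when its lifetime runs out.
; A hit on the Collider component applies a fixed amount of damage to the other actor, then destroys the projectile.
; Tick accumulates elapsed time in DureeDeVie and destroys the actor once it exceeds EsperanceDeVie.
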(event OnComponentHit(Collider)
  (params (HitComponent :type Primitive%20Component%20Object%20Reference) (OtherActor :type Actor%20Object%20Reference) (OtherComp :type Primitive%20Component%20Object%20Reference) (NormalImpulse :type Vector :default "0, 0, 0") (Hit :type Hit%20Result%20Structure%20%28by%20ref%29))
  ;[1 0.1469 0] Collision
  (Game|Damage|ApplyDamage OtherActor 1.0 0 0)
  (Actor|DestroyActor))

(event EventBeginPlay)

(event Collision|EventActorBeginOverlap
  (params (OtherActor :type Actor%20Object%20Reference)))

(event EventTick
  (params (DeltaSeconds :type Float%20%28single-precision%29))
  ;[0 0 0] AutoDestruction en fonction du temps
  (Variables|Default|SetDuree_de_vie (+ DeltaSeconds (Variables|Default|GetDuree_de_vie)))
  (if (> (Variables|Default|GetDuree_de_vie) (Variables|Default|GetEsperance_de_vie))
    (Actor|DestroyActor)))

(fn ConstructionScript)